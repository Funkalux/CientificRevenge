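; Player character steered by press-and-drag, which shows the failure menu on overlapping a Guard.
; BeginPlay sets walk speed and adds the main game UI unless CurrentLevel is 0.
; While pressed, Tick projects press and current mouse positions onto the Z=0 plane, using their offset as an analog stick scaled by MaxDistance.
; A zero offset moves the player at full input in the last direction.
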(event EventTick
  (params (DeltaSeconds :type Float%20%28single-precision%29))
  (bind _position (Utilities|GetClickPosition false))
  (bind _touch_begin_location (Variables|Default|GetTouch%20Begin%20Location))
  (bind _returnvalue (Utilities|ScreentoWorldPos _position))
  (bind _returnvalue_2 (Utilities|ScreentoWorldPos _touch_begin_location))
  (bind _returnvalue_3 (- _returnvalue _returnvalue_2))
  (bind _returnvalue_4 (Math|Vector2D|Vector2DLength _returnvalue_3))
  (bind _returnvalue_5 (Math|Vector2D|Normalize2D _returnvalue_3))
  ;[1 0.01891 0] Move Character taking a Screen Space Vector
  (if (Variables|Default|GetShould%20Move)
    (if (== _returnvalue_4 0.0)
      (Pawn|Input|AddMovementInput (Math|Conversions|ToVector(Vector2D) (Variables|Default|GetLastDirection)) 1.0 false)
      (else
        (Variables|Default|SetLastDirection _returnvalue_5)
        (Pawn|Input|AddMovementInput (Math|Conversions|ToVector(Vector2D) _returnvalue_5) (Math|Float|Clamp(Float) (/ _returnvalue_4 (Variables|Default|GetMaxDistance))) false)))))

(event EventBeginPlay
  ;[0 1 0.07707] Set Initial Walk Speed
  (Variables|/Script/Engine.CharacterMovementComponent|SetMaxWalkSpeed (Variables|Character|GetCharacterMovement) (Variables|Default|GetMax%20Movement%20Speed))
  (bind _returnvalue (UserInterface|CreateWidget "/Game/UI/MainGameUI.MainGameUI_C"))
  (if (!= (Variables|Default|GetCurrentLevel) 0)
    (UserInterface|Viewport|AddtoViewport _returnvalue 0)))

(event Collision|EventActorBeginOverlap
  (params (OtherActor :type Actor%20Object%20Reference))
  ;[1 1 1] Comment
  (Utilities|Casting|CastToGuard OtherActor)
  (Default|ShowFailureMenu (Variables|Default|GetUI)))

(event Input|ActionEvents|InputActionTouchAction
  (params (Key :type Key%20Structure :default "None"))
  ;[1 0.8106 0] Get Screen Input
  (:Pressed
    (Variables|Default|SetShould%20Move true)
    (Variables|Default|SetTouch%20Begin%20Location (Utilities|GetClickPosition false)))
  (:Released
    (Variables|Default|SetShould%20Move false)))

(fn ConstructionScript)