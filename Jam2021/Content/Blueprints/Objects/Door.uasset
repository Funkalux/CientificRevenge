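; Door actor that works as a level exit, swinging open when the player touches it and loading the level named by LevelName.
; On the first player overlap it rotates both meshes, stops player walking and starts an audio-visual fade-out.
; Tick then runs OpeningCountDown and opens the level once it drops below zero.
; Ending a player overlap rotates the meshes back without clearing IsOpen.
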(event EventBeginPlay
  (Transformation|AddRelativeRotation (Variables|Default|GetStaticMesh) "0,229.500000, 0" false false)
  (Transformation|AddRelativeRotation (Variables|Default|GetStaticMesh2) "0,229.500000, 0" false false))

(event Collision|EventActorBeginOverlap
  (params (OtherActor :type Actor%20Object%20Reference))
  (Audio|PlaySoundatLocation "/Game/Sound/DoorOpenSound.DoorOpenSound" (Transformation|GetActorLocation self) "0, 0, 0" 1.0 1.0 0.0 0 0 0)
  (if (not (Variables|Default|GetisOpen))
    (bind _asplayer (Utilities|Casting|CastToPlayer OtherActor))
    (Variables|Default|SetisOpen true)
    (Variables|/Script/Engine.CharacterMovementComponent|SetMaxWalkSpeed (Variables|/Script/Engine.Character|GetCharacterMovement _asplayer) 0.0)
    (Transformation|AddRelativeRotation (Variables|Default|GetStaticMesh) "0,130.500000, 0" false false)
    (Transformation|AddRelativeRotation (Variables|Default|GetStaticMesh2) "0,130.500000, 0" false false)
    (CameraFades|StartCameraFade :self (Game|GetPlayerCameraManager 0) :ToAlpha 1.0 :Duration 1.0 :bShouldFadeAudio true :bHoldWhenFinished true)))

(event Collision|EventActorEndOverlap
  (params (OtherActor :type Actor%20Object%20Reference))
  (Audio|PlaySoundatLocation 0 (Transformation|GetActorLocation) "0, 0, 0" 1.0 1.0 0.0 0 0 0)
  (Utilities|Casting|CastToPlayer OtherActor)
  (Transformation|AddRelativeRotation (Variables|Default|GetStaticMesh) "0,-130.500000, 0" false false)
  (Transformation|AddRelativeRotation (Variables|Default|GetStaticMesh2) "0,-130.500000, 0" false false))

(event EventTick
  (params (DeltaSeconds :type Float%20%28single-precision%29))
  (if (Variables|Default|GetisOpen)
    (bind _output_get (Variables|Default|SetOpeningCountDown (- (Variables|Default|GetOpeningCountDown) DeltaSeconds)))
    (if (< _output_get 0.0)
      (Game|OpenLevel(byName) (Variables|Default|GetLevel%20Name)))))

(fn ConstructionScript)