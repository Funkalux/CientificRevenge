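; MediumObject is a medium-tier object Blueprint that carries a randomized point value and one of several lab-prop looks.
; Its construction script adds a random integer to PointsValue and randomly picks the Mesh from a vial, two kinds of weighs and a device.
; The event graph holds only disabled default events, so the Blueprint adds no runtime logic of its own.
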(event EventBeginPlay
  (|CallParentFunction) ; This node is disabled and will not be called.\nDrag off pins to build functionality.
)

(event Collision|EventActorBeginOverlap
  (params (OtherActor :type Actor%20Object%20Reference))
  (|CallParentFunction OtherActor) ; This node is disabled and will not be called.\nDrag off pins to build functionality.
)

(event EventTick
  (params (DeltaSeconds :type Float%20%28single-precision%29)))

(fn ConstructionScript
  (Variables|Default|SetPointsValue (+ (Variables|Default|GetPointsValue) (Math|Random|RandomIntegerinRange 25 40)))
  (Variables|Default|SetMesh (Utilities|Select :Index (Math|Random|RandomIntegerinRange 0 3) :Option%200 "/Game/Assets/vial.vial" :Option%201 "/Game/Assets/weighs.weighs" :Option%202 "/Game/Assets/device_Device.device_Device" :Option%203 "/Game/Assets/weighs_electronic.weighs_electronic")))