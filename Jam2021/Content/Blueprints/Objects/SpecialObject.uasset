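; SpecialObject is an object Blueprint that randomizes its point value and its look, choosing between microscope and centrifuge meshes.
; The Construction Script adds a small random integer bonus to PointsValue and sets Mesh from a random two-way select.
; The Event Graph holds only disabled default events, so the Blueprint adds no runtime logic of its own.
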(event EventBeginPlay
  (|CallParentFunction) ; This node is disabled and will not be called.\nDrag off pins to build functionality.
)

(event Collision|EventActorBeginOverlap
  (params (OtherActor :type Actor%20Object%20Reference))
  (|CallParentFunction OtherActor) ; This node is disabled and will not be called.\nDrag off pins to build functionality.
)

(event EventTick
  (params (DeltaSeconds :type Float%20%28single-precision%29)))

(fn ConstructionScript
  (Variables|Default|SetPointsValue (+ (Variables|Default|GetPointsValue) (Math|Random|RandomIntegerinRange 0 10)))
  (Variables|Default|SetMesh (Utilities|Select :Index (Math|Random|RandomIntegerinRange 0 1) :Option%200 "/Game/Assets/microscope_Microscope.microscope_Microscope" :Option%201 "/Game/Assets/centrifuge.centrifuge")))