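; GenericObject is a collectible with a configurable mesh that adds PointsValue to the Player's Points on overlap.
; BeginPlay applies the mesh, and the overlap starts a timeline that spins it, scales it cumulatively and offsets it.
; The per-frame offset uses the Player's absolute X/Y and a JumpHeight-scaled Z, times delta time.
; A one-second Delay on the timeline's Update then destroys the actor.
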(event EventBeginPlay
  (Components|StaticMesh|SetStaticMesh (Variables|Default|GetObject_Mesh) (Variables|Default|GetMesh)))

(event Collision|EventActorBeginOverlap
  (params (OtherActor :type Actor%20Object%20Reference))
  (bind _asplayer (Utilities|Casting|CastToPlayer OtherActor))
  (Variables|/Game/Blueprints/Player/Player.Player_C|SetPoints _asplayer (+ (Variables|/Game/Blueprints/Player/Player.Player_C|GetPoints _asplayer) (Variables|Default|GetPointsValue)))
  (bind (_direction _newtrack_0 _newtrack_1 _newtrack_2) (Timeline|Rotate_and_shrink Play)
    (:Update
      (Transformation|AddRelativeLocation (Variables|Default|GetObject_Mesh) (* (Math|Vector|MakeVector (.X (Math|Vector|BreakVector (Transformation|GetActorLocation _asplayer))) (.Y (Math|Vector|BreakVector (Transformation|GetActorLocation _asplayer))) (* (Variables|Default|Getjump_height) _newtrack_2)) (Utilities|Time|GetWorldDeltaSeconds)) false false)
      (Transformation|SetWorldRotation (Variables|Default|GetObject_Mesh) (Math|Rotator|Lerp(Rotator) "0, 0, 0" "180.000000,360.000000,60.000000" _newtrack_0) false false)
      (Transformation|SetWorldScale3D (Variables|Default|GetObject_Mesh) (* (Math|Vector|MakeVector _newtrack_1 _newtrack_1 _newtrack_1) (Transformation|GetWorldScale (Variables|Default|GetObject_Mesh))))
      (Utilities|FlowControl|Delay 1.0)
      (Actor|DestroyActor))))

(fn ConstructionScript)