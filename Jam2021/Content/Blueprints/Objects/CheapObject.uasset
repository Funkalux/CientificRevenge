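; CheapObject is a low-value object Blueprint worth a fixed number of points, with a randomly chosen appearance.
; Its construction script sets the points, picks one of several bottle, flower and lab furniture meshes at random, and writes the value into a hidden point text component.
; BeginPlay and overlap events only call the parent class, and Tick is empty.
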(event EventBeginPlay
  (|CallParentFunction))

(event Collision|EventActorBeginOverlap
  (params (OtherActor :type Actor%20Object%20Reference))
  (|CallParentFunction OtherActor))

(event EventTick
  (params (DeltaSeconds :type Float%20%28single-precision%29)))

(fn ConstructionScript
  (Rendering|SetVisibility (Variables|Default|GetPointValue) false false)
  (bind _output_get (Variables|Default|SetPointsValue 10))
  (Variables|Default|SetMesh (Utilities|Select :Index (Math|Random|RandomIntegerinRange 0 5) :Option%200 "/Game/Assets/bottle_Bottle_1.bottle_Bottle_1" :Option%201 "/Game/Assets/bottle_Bottle_2.bottle_Bottle_2" :Option%202 "/Game/Assets/flower.flower" :Option%203 "/Game/Assets/lab_table_Lab_table.lab_table_Lab_table" :Option%204 "/Game/Assets/lab_chair_Lab_chair_base.lab_chair_Lab_chair_base" :Option%205 "/Game/Assets/lab_chair_Lab_chair_seat.lab_chair_Lab_chair_seat"))
  (bind _output_get_2 (Variables|Default|SetPointText (Utilities|Text|ToText(String) (Utilities|String|ToString(Integer) _output_get))))
  (Rendering|Components|TextRender|SetText (Variables|Default|GetPointValue) _output_get_2))